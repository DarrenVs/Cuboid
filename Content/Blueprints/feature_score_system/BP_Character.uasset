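; BP_Character is a test Blueprint for a persistent score system.
; On BeginPlay it loads the BP_Save_Data save from the "data" slot and copies ScoreSaved into Score.
; Pressing Space Bar adds a fixed amount to Score, writes it into a newly created save object, prints it and saves it back to that slot.
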(event EventBeginPlay
  (bind _returnvalue (SaveGame|LoadGamefromSlot "data"))
  (bind _asbp_save_data (Utilities|Casting|CastToBP_Save_Data _returnvalue))
  (Variables|Default|Setscore (Variables|/Game/Blueprints/feature_score_system/BP_Save_Data.BP_Save_Data_C|Getscore_saved _asbp_save_data)))

(event Collision|EventActorBeginOverlap
  (params (OtherActor :type Actor%20Object%20Reference)))

(event EventTick
  (params (DeltaSeconds :type Float%20%28single-precision%29)))

(event Input|KeyboardEvents|SpaceBar
  (params (Key :type Key%20Structure))
  (:Pressed
    (Variables|Default|Setscore (+ (Variables|Default|Getscore) 1000))
    (bind _returnvalue (SaveGame|CreateSaveGameObject "/Game/Blueprints/feature_score_system/BP_Save_Data.BP_Save_Data_C"))
    (bind _asbp_save_data (Utilities|Casting|CastToBP_Save_Data _returnvalue))
    (bind _output_get (Variables|/Game/Blueprints/feature_score_system/BP_Save_Data.BP_Save_Data_C|Setscore_saved _asbp_save_data (Variables|Default|Getscore)))
    (Development|PrintString (Utilities|String|ToString(Integer) _output_get))
    (SaveGame|SaveGametoSlot _returnvalue "data")))

(fn ConstructionScript)