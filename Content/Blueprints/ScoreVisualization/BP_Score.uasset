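; BP_Score is a prototype scoreboard actor that draws a score screen into a canvas render target.
; BeginPlay creates the target, binds its update event and refreshes it.
; The update draws a background texture and placeholder test text; no score value is read.
; The nodes that would apply the target to the Scoreboard through a dynamic M_ScoreScreen material are unconnected, so this graph never displays it there.
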(event Custom|CustomEvent_0
  (params (Canvas :type Canvas%20Object%20Reference) (Width :type Integer) (Height :type Integer))
  (Canvas|DrawTexture :self Canvas :RenderTexture "/Game/Effects/Textures/Misc/1479530916-Don-Diablo-copy_png.1479530916-Don-Diablo-copy_png" :ScreenSize (Math|Vector2D|MakeVector2D (Math|Conversions|ToFloat(Integer) Width) (Math|Conversions|ToFloat(Integer) Height)) :BlendMode "BLEND_Opaque")
  (HUD|DrawText Canvas "/Game/Fonts/ScoreFont.ScoreFont" "TEST TEST TEST" "(X=15.000000,Y=15.000000)" "(R=1.000000,G=1.000000,B=1.000000,A=1.000000)" 0.0 "(R=0.000000,G=0.000000,B=0.000000,A=1.000000)" "(X=1.000,Y=1.000)" false false false "(R=0.000000,G=0.000000,B=0.000000,A=1.000000)"))

(event Collision|EventActorBeginOverlap
  (params (OtherActor :type Actor%20Object%20Reference)))

(event EventTick
  (params (DeltaSeconds :type Float%20%28single-precision%29)))

(event EventBeginPlay
  (bind _returnvalue (CanvasRenderTarget2D|CreateCanvasRenderTarget2D "/Script/Engine.CanvasRenderTarget2D" 1024 1024))
  (bind _output_get (Variables|Default|SetTexture _returnvalue))
  (EventDispatchers|BindEventtoOnCanvasRenderTargetUpdate _output_get (delegate Custom|CustomEvent_0))
  (Class|CanvasRenderTarget2D|UpdateResource _output_get))

(fn ConstructionScript)