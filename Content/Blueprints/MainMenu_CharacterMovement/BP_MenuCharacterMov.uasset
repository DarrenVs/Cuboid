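; Main menu actor that flies the Don character along a spline for the door intro.
; Once StartMoving is set (by BP_MainMenu, per its comment), Tick swaps the T-pose Don for the flying model and activates the jet sound.
; Each tick adds Speed plus scaled game time to the spline distance, so movement accelerates and is frame-rate dependent, then updates location and rotation from the spline.
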(event EventTick
  (params (DeltaSeconds :type Float%20%28single-precision%29))
  (bind _splineobj (Variables|Default|GetSplineObj))
  (bind _donmodel (Variables|Default|GetDonModel))
  ;[1 1 1] Set the start moving in the BP_MainMenu
  (if (Variables|Default|GetStartMoving)
    ;[1 1 1] Set the Tpos Don off and the flying on. Start the jet sound
    (Rendering|SetActorHiddenInGame (Variables|Default|GetDonModel) false)
    (Rendering|SetActorHiddenInGame (Variables|Default|GetTPoseDon) true)
    (Components|Activation|Activate (Variables|/Script/Engine.AmbientSound|GetAudioComponent (Variables|Default|GetFlyingSound)) false)
    ;[1 1 1] Move Don along a spline for Door intro.
    (bind _output_get (Variables|Default|SetSplineDistance (+ (* (Utilities|Time|GetTimeSeconds) 0.5) (Variables|Default|GetSpeed) (Variables|Default|GetSplineDistance))))
    (Transformation|SetActorLocation _donmodel (Spline|GetLocationatDistanceAlongSpline _splineobj _output_get "World") false false)
    (Transformation|SetActorRotation _donmodel (Spline|GetRotationatDistanceAlongSpline _splineobj _output_get "Local"))))

(fn ConstructionScript)