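; Manager actor that builds and recycles a row of moving Chunk actors along the X axis.
; On BeginPlay it spawns the chunks end to end, starting one chunk length behind the world origin, passing each a manager reference, its index and the shared speed.
; RespawnChunk reuses a chunk by ID, moving it to the last slot's position and calling its Respawn rather than spawning a new actor.
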(event Custom|CreateChunk
  (bind _chunklength (Variables|Default|GetChunkLength))
  (bind _returnvalue (Game|SpawnActorfromClass (Variables|Default|GetChunk) (Math|Transform|MakeTransform (Math|Vector|MakeVector (Math|Conversions|ToFloat(Integer) (- (* (Utilities|Array|Length (Variables|Default|GetChunks)) _chunklength) _chunklength)) 0.0 0.0)) "Undefined" 0 self (Utilities|Array|Length (Variables|Default|GetChunks)) (Variables|Default|GetChunkSpeed) 0))
  (Utilities|Array|Add (Variables|Default|GetChunks) _returnvalue))

(event Custom|RespawnChunk
  (params (ChunkID :type Integer))
  (bind _chunklength (Variables|Default|GetChunkLength))
  (bind _chunks (Variables|Default|GetChunks))
  (bind _output (Utilities|Array|Get(acopy) _chunks ChunkID))
  (Transformation|SetActorLocation _output (Math|Vector|MakeVector (Math|Conversions|ToFloat(Integer) (- (* (- (Utilities|Array|Length (Variables|Default|GetChunks)) 1) _chunklength) _chunklength)) 0.0 0.0) false false)
  (Default|Respawn _output))

(event EventBeginPlay
  (for _index (range 0 (Variables|Default|GetChunkAmount))
    (CallFunction|CreateChunk)))

(event Collision|EventActorBeginOverlap
  (params (OtherActor :type Actor%20Object%20Reference)))

(event EventTick
  (params (DeltaSeconds :type Float%20%28single-precision%29)))

(fn ConstructionScript)