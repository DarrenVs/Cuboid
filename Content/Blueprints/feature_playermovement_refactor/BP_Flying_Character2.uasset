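; Flying player character that moves a physics-driven capsule along the Y and Z axes from flying control input.
; Each Tick lerps the input into a clamped flying delta for smoothing, then adds it, scaled by flying speed, to the capsule's velocity.
; Velocity is lerped toward zero as drag before being applied as physics linear velocity, and capsule rotation is reset to zero.
; Actor overlap only prints a debug "Hello".
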(event EventBeginPlay)

(event Collision|EventActorBeginOverlap
  (params (OtherActor :type Actor%20Object%20Reference))
  (Development|PrintString "Hello"))

(event EventTick
  (params (DeltaSeconds :type Float%20%28single-precision%29))
  ;[0.08994 0.03546 0.1146] Calc input delta
  ;;[0 0 0] Set new flying delta
  (Variables|Default|SetFlying%20Delta (Math|Vector|ClampVectorSize (Math|Vector|Lerp(Vector) (Variables|Default|GetFlying%20Delta) (Math|Vector|MakeVector 0.0 (Input|AxisValues|GetFlyingControls_X) (Input|AxisValues|GetFlyingControls_Y)) (Variables|Default|GetFlying%20Delta%20Drag)) 0.0 (Variables|Default|GetFlying%20Delta%20Max)))
  ;[0.04191 0.1354 0.08254] Set velocity
  (Physics|SetPhysicsLinearVelocity (Variables|Default|GetCapsule) (Math|Vector|Lerp(Vector) (+ (Transformation|GetComponentVelocity (Variables|Default|GetCapsule)) (* (Math|Vector|Normalize (Variables|Default|GetFlying%20Delta)) (* (Math|Float|Clamp(Float) (Math|Vector|VectorLength (Variables|Default|GetFlying%20Delta))) (Variables|Default|GetFlying%20Speed)))) "0, 0, 0" (Variables|Default|GetVelocity%20Drag)) false "None")
  ;[0.04191 0.1354 0.08254] Freeze rotation
  (Transformation|SetWorldRotation (Variables|Default|GetCapsule) "0, 0, 0" false false))

(fn ConstructionScript)