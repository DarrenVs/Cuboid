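; BP_BuildingManager is a building catalog that supplies meshes and materials for four building types, A through D.
; Each type has its own array of entries pairing a BuildingMesh with a BuildingMaterial.
; ReturnBuilding switches on the type and returns a randomly indexed mesh and material from that array, while ReturnAllBuildings returns the whole array.
; The event graph and construction script are empty, so it acts only when called.
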(event EventBeginPlay)

(event Collision|EventActorBeginOverlap
  (params (OtherActor :type Actor%20Object%20Reference)))

(event EventTick
  (params (DeltaSeconds :type Float%20%28single-precision%29)))

(fn ConstructionScript)

(fn ReturnBuilding
  (params (NewParam :type ObstacleIndex%20Enum :default "NewEnumerator0"))
  (bind _buildingclass_a (Variables|Default|GetBuildingClass_A))
  (bind _buildingclass_b (Variables|Default|GetBuildingClass_B))
  (bind _buildingclass_c (Variables|Default|GetBuildingClass_C))
  (bind _buildingclass_d (Variables|Default|GetBuildingClass_D))
  (bind _returnvalue (Utilities|Array|Length _buildingclass_d))
  (bind _returnvalue_2 (Utilities|Array|Length _buildingclass_a))
  (bind _returnvalue_3 (Utilities|Array|Length _buildingclass_b))
  (bind _returnvalue_4 (Utilities|Array|Length _buildingclass_c))
  (bind _returnvalue_5 (- _returnvalue_4 1))
  (bind _returnvalue_6 (- _returnvalue 1))
  (bind _returnvalue_7 (- _returnvalue_2 1))
  (bind _returnvalue_8 (- _returnvalue_3 1))
  (bind _returnvalue_9 (Math|Random|RandomIntegerinRange 0 _returnvalue_6))
  (bind _returnvalue_10 (Math|Random|RandomIntegerinRange 0 _returnvalue_7))
  (bind _returnvalue_11 (Math|Random|RandomIntegerinRange 0 _returnvalue_8))
  (bind _returnvalue_12 (Math|Random|RandomIntegerinRange 0 _returnvalue_5))
  (bind _output (Utilities|Array|Get(acopy) _buildingclass_d _returnvalue_9))
  (bind _output_2 (Utilities|Array|Get(acopy) _buildingclass_a _returnvalue_10))
  (bind _output_3 (Utilities|Array|Get(acopy) _buildingclass_b _returnvalue_11))
  (bind _output_4 (Utilities|Array|Get(acopy) _buildingclass_c _returnvalue_12))
  (switch Utilities|FlowControl|Switch|SwitchonObstacleIndex NewParam
    (:NewEnumerator0
      (return (.buildingmesh _output_2) (.buildingmaterial _output_2)))
    (:NewEnumerator1
      (return (.buildingmesh _output_3) (.buildingmaterial _output_3)))
    (:NewEnumerator2
      (return (.buildingmesh _output_4) (.buildingmaterial _output_4)))
    (:NewEnumerator3
      (return (.buildingmesh _output) (.buildingmaterial _output)))))

(fn ReturnAllBuildings
  (params (BuildingType :type ObstacleIndex%20Enum :default "NewEnumerator0"))
  (return (Utilities|Select :Index BuildingType :NewEnumerator0 (Variables|Default|GetBuildingClass_A) :NewEnumerator1 (Variables|Default|GetBuildingClass_B) :NewEnumerator2 (Variables|Default|GetBuildingClass_C) :NewEnumerator3 (Variables|Default|GetBuildingClass_D))))