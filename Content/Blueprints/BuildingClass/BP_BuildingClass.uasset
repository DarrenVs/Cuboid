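; Music-reactive building actor that takes its mesh and material for its BuildingType from BP_BuildingManager at BeginPlay.
; InteractionOnMusic picks an audio band by InteractionType: Bass scales the actor, Frequencty offsets it along its up vector, Voice jumps Z above a threshold or eases back.
; Those three bands also drive the dynamic material's glow Intensity.
; Snare only sets the array index, and DiscoColors is disconnected.
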(event EventBeginPlay
  (bind _material (CallFunction|SpawnBuilding (Variables|Default|GetBuildingType)))
  ;[1 1 1] Start pos for original Z.
  (Variables|Default|SetStartingTransform (Transformation|GetRelativeTransform (Variables|Default|GetStaticMesh)))
  (bind _returnvalue (Rendering|Material|CreateDynamicMaterialInstance (Variables|Default|GetStaticMesh) 0 _material :!class /Script/Engine.PrimitiveComponent))
  (Variables|Default|SetMaterialRef _returnvalue))

(fn ConstructionScript)

(fn InteractiononMusic
  (params (AudioValues :type Array%20of%20Floats%20%28single-precision%29))
  (bind _startingtransform (Variables|Default|GetStartingTransform))
  (bind _staticmesh (Variables|Default|GetStaticMesh))
  (bind (_location _rotation _scale) (Math|Transform|BreakTransform _startingtransform))
  (bind _returnvalue (Transformation|GetRelativeTransform _staticmesh))
  (bind _location_2 (Math|Transform|BreakTransform _returnvalue))
  (bind _z (Math|Vector|BreakVector _location))
  ;[1 1 1] What music stuff do I interact with?
  (switch Utilities|FlowControl|Switch|SwitchonInteractionIndex (Variables|Default|GetInteractionType)
    (:NewEnumerator0
      (Variables|Default|SetMusicArrayIndex 0)
      (CallFunction|ScaleonMusic (/ (Math|Float|Clamp(Float) (Utilities|Array|Get(acopy) AudioValues (Variables|Default|GetMusicArrayIndex)) -2e+02 2e+02) (Variables|Default|GetDamping)) (.X (Math|Vector|BreakVector _scale)))
      (Rendering|Material|SetScalarParameterValue (Variables|Default|GetMaterialRef) "Intensity" (* (Math|Float|Clamp(Float) (Utilities|Array|Get(acopy) AudioValues (Variables|Default|GetMusicArrayIndex)) -2e+02 2e+02) (Variables|Default|GetGlowIntensity)) :!class /Script/Engine.MaterialInstanceDynamic :!label _label))
    (:NewEnumerator1
      (Variables|Default|SetMusicArrayIndex 1)
      (CallFunction|MoveZ _location_2 _location (/ (Math|Float|Clamp(Float) (Utilities|Array|Get(acopy) AudioValues (Variables|Default|GetMusicArrayIndex)) -2e+02 2e+02) (Variables|Default|GetDamping)) _z _rotation)
      (goto _label))
    (:NewEnumerator2
      (Variables|Default|SetMusicArrayIndex 2)
      (CallFunction|AggresiveAttack _location_2 (/ (Math|Float|Clamp(Float) (Utilities|Array|Get(acopy) AudioValues (Variables|Default|GetMusicArrayIndex)) -2e+02 2e+02) (Variables|Default|GetDamping)) _z)
      (goto _label))
    (:NewEnumerator3
      (Variables|Default|SetMusicArrayIndex 3))))

(fn MoveZ
  (params (ObjectVector :type Vector) (OldPosition :type Vector) (MusicValue :type Float%20%28single-precision%29) (MinimalZPos :type Float%20%28single-precision%29) (StartRotation :type Rotator))
  (Transformation|SetActorRelativeLocation (+ (* (Math|Conversions|ToVector(Float) MusicValue) (Math|Vector|GetUpVector StartRotation)) OldPosition)))

(fn ScaleonMusic
  (params (MusicValues :type Float%20%28single-precision%29) (MInimalScale :type Float%20%28single-precision%29))
  (Development|PrintString (Utilities|String|ToString(Float) MusicValues))
  ;[1 1 1] scale
  (Transformation|SetActorScale3D (Math|Conversions|ToVector(Float) (Math|Float|Clamp(Float) MusicValues MInimalScale (Variables|Default|GetMaxScale)))))

(fn AggresiveAttack
  (params (ObjectVector :type Vector) (MusicValues :type Float%20%28single-precision%29) (MinimalZPos :type Float%20%28single-precision%29))
  (bind (_x _y _z) (Math|Vector|BreakVector ObjectVector))
  (bind (_x_2 _y_2 _z_2) (Math|Vector|BreakVector ObjectVector))
  ;[1 1 1] Check if the music value is higher than minimal attack value.
  (if (>= MusicValues (Variables|Default|GetMinAggressionAttackValue))
    ;[1 1 1] Move Z attack
    (Transformation|SetActorLocation (Math|Vector|MakeVector _x_2 _y_2 (Math|Float|Clamp(Float) (+ _z_2 MusicValues) MinimalZPos 6e+02)) false false)
    (else
      ;[1 1 1] Move Z back to start positionZ
      (Transformation|SetActorLocation (Math|Vector|MakeVector _x _y (Math|Float|Lerp _z MinimalZPos 0.5)) false false))))

(fn DiscoColors
  (params (MusicParamaters :type Array%20of%20Floats%20%28single-precision%29)))

(fn SpawnBuilding
  (params (TypeBuildingWanted :type ObstacleIndex%20Enum :default "NewEnumerator0"))
  (bind _outactors (Actor|GetAllActorsOfClass "/Game/Blueprints/BuildingClass/BP_BuildingManager.BP_BuildingManager_C"))
  (bind (_building _material) (Default|ReturnBuilding _outactors TypeBuildingWanted))
  (Components|StaticMesh|SetStaticMesh (Variables|Default|GetStaticMesh) _building)
  (return _material))