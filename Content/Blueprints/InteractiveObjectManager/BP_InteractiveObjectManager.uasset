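; BP_InteractiveObjectManager keeps a list of BP_BuildingClass actors and makes them react to music.
; UpdateArray appends every such actor in the level to InteractableObjects without clearing it, and is meant to run after chunk build or destruction.
; MoveObjects passes MusicParameters to each object's InteractionOnMusic, or only fills the list when it is empty.
; Its event graph is unused, so both functions rely on external callers.
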(event EventBeginPlay)

(event Collision|EventActorBeginOverlap
  (params (OtherActor :type Actor%20Object%20Reference)))

(event EventTick
  (params (DeltaSeconds :type Float%20%28single-precision%29)))

(fn ConstructionScript)

(fn UpdateArray
  ;[1 1 1] Call this after build/destruction of a chunk.
  (bind _outactors (Actor|GetAllActorsOfClass "/Game/Blueprints/ActorClass/BP_BuildingClass.BP_BuildingClass_C"))
  (for _array_element _outactors
    (Utilities|Array|Add (Variables|Default|GetInteractableObjects) _array_element)))

(fn MoveObjects
  (params (MusicParameters :type Array%20of%20Floats%20%28single-precision%29))
  (bind _interactableobjects (Variables|Default|GetInteractableObjects))
  ;[1 1 1] Are there interactive objects in the scene?
  (if (> (Math|Conversions|ToFloat(Integer) (Utilities|Array|Length _interactableobjects)) 0.0)
    (for _array_element _interactableobjects
      (Default|InteractiononMusic _array_element MusicParameters))
    (else
      (CallFunction|UpdateArray))))