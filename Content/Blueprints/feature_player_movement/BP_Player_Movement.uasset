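; BP_Player_Movement is a VR player Blueprint that, despite its name, only sets up the camera and runs a gaze trace, with no movement logic.
; BeginPlay sets an eye-level tracking origin and moves VRCameraRoot to the CameraHeight offset.
; Each Tick line-traces 1500 units along the VR camera's forward vector against WorldStatic objects, draws it for debugging and prints the hit location off-screen.
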(event EventBeginPlay
  (Class|HeadMountedDisplayFunctionLibrary|SetTrackingOrigin "Eye")
  (Transformation|SetRelativeLocation (Variables|Default|GetVRCameraRoot) (Variables|Default|GetCameraHeight) false false))

(event Collision|EventActorBeginOverlap
  (params (OtherActor :type Actor%20Object%20Reference)))

(event EventTick
  (params (DeltaSeconds :type Float%20%28single-precision%29))
  (bind _vrcamera (Variables|Default|GetVRCamera))
  (bind _returnvalue (Transformation|GetWorldLocation _vrcamera))
  (bind _outhit (Collision|LineTraceForObjects _returnvalue (+ _returnvalue (* (Math|Vector|GetForwardVector (Transformation|GetWorldRotation _vrcamera)) 1.5e+03)) (Utilities|Array|MakeArray "ObjectTypeQuery1") false 0 "ForOneFrame"))
  (Development|PrintString (Utilities|String|ToString(Vector) (.Location (Collision|BreakHitResult _outhit))) false))

(fn ConstructionScript)