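; VR camera actor that steers the player by gaze.
; On start it sets eye-level tracking and offsets the camera root by a height setting.
; Each tick it traces a long, debug-drawn object ray along the camera's forward vector.
; On a blocking hit, it moves the first BP_PlayerBehaviour actor using VInterpTo toward the hit point, starting from the player's Y and Z with X zeroed.
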(event EventBeginPlay
  ;[1 1 1] VR Camera Behaviour
  (Class|HeadMountedDisplayFunctionLibrary|SetTrackingOrigin "Eye")
  (Transformation|SetRelativeLocation (Variables|Default|GetVRCameraRoot) (Variables|Default|GetCameraHeight) false false))

(event Collision|EventActorBeginOverlap
  (params (OtherActor :type Actor%20Object%20Reference)))

(event EventTick
  (params (DeltaSeconds :type Float%20%28single-precision%29))
  (bind _vrcamera (Variables|Default|GetVRCamera))
  (bind _returnvalue (Transformation|GetWorldLocation _vrcamera))
  ;[1 1 1] 'Update' Function
  ;[1 1 1] drawing line for collision
  (bind _outhit (Collision|LineTraceForObjects _returnvalue (+ _returnvalue (* (Math|Vector|GetForwardVector (Transformation|GetWorldRotation _vrcamera)) 9e+03)) (Utilities|Array|MakeArray "ObjectTypeQuery7") false 0 "ForOneFrame"))
  (if (.bBlockingHit (Collision|BreakHitResult _outhit))
    (bind _output_get (Variables|Default|SetRayCastCollisionLocation (.Location (Collision|BreakHitResult _outhit))))
    ;[1 1 1] Getting Object with Blueprint reference
    (bind _outactors (Actor|GetAllActorsOfClass "/Game/Blueprints/feature_player_movement/BP_PlayerBehaviour.BP_PlayerBehaviour_C"))
    ;[1 1 1] Casting The movement behaviour to actor (player)
    (bind _asbp_player_behaviour (Utilities|Casting|CastToBP_PlayerBehaviour (Utilities|Array|Get(acopy) _outactors)))
    (Transformation|SetActorLocation _asbp_player_behaviour (Math|Interpolation|VInterpTo (Math|Vector|MakeVector 0.0 (.Y (Math|Vector|BreakVector (Transformation|GetWorldLocation (Variables|/Game/Blueprints/feature_player_movement/BP_PlayerBehaviour.BP_PlayerBehaviour_C|GetPlayer _asbp_player_behaviour)))) (.Z (Math|Vector|BreakVector (Transformation|GetWorldLocation (Variables|/Game/Blueprints/feature_player_movement/BP_PlayerBehaviour.BP_PlayerBehaviour_C|GetPlayer _asbp_player_behaviour))))) _output_get DeltaSeconds 1.0) false false)))

(fn ConstructionScript)