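; Music-reactive building actor that changes its transform and material glow from an array of audio values.
; BeginPlay caches the mesh's relative transform and creates a dynamic material for glow.
; InteractionOnMusic picks an audio band by InteractionType: Bass scales the actor, Voice lifts it above a threshold or eases it back, and all but Snare drive Intensity.
; Frequency's MoveZ ignores the music value, and Snare only sets the array index.
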(event EventBeginPlay
  (bind _staticmesh (Variables|Default|GetStaticMesh))
  ;[1 1 1] Start pos for original Z.
  (Variables|Default|SetStartingTransform (Transformation|GetRelativeTransform (Variables|Default|GetStaticMesh)))
  (bind _returnvalue (Rendering|Material|CreateDynamicMaterialInstance _staticmesh 0 (Rendering|Material|GetMaterial _staticmesh 0) :!class /Script/Engine.PrimitiveComponent))
  (Variables|Default|SetIntensity _returnvalue))

(event Collision|EventActorBeginOverlap
  (params (OtherActor :type Actor%20Object%20Reference)))

(event EventTick
  (params (DeltaSeconds :type Float%20%28single-precision%29)))

(fn ConstructionScript)

(fn InteractiononMusic
  (params (AudioValues :type Array%20of%20Floats%20%28single-precision%29))
  (bind _startingtransform (Variables|Default|GetStartingTransform))
  (bind _staticmesh (Variables|Default|GetStaticMesh))
  (bind (_location _rotation _scale) (Math|Transform|BreakTransform _startingtransform))
  (bind _returnvalue (Transformation|GetRelativeTransform _staticmesh))
  (bind _location_2 (Math|Transform|BreakTransform _returnvalue))
  (bind _z (Math|Vector|BreakVector _location))
  ;[1 1 1] What music stuff do I interact with?
  (switch Utilities|FlowControl|Switch|SwitchonInteractionIndex (Variables|Default|GetInteractionType)
    (:NewEnumerator0
      (Variables|Default|SetMusicArrayIndex 0)
      (CallFunction|ScaleonMusic (/ (Math|Float|Clamp(Float) (Utilities|Array|Get(acopy) AudioValues (Variables|Default|GetMusicArrayIndex)) -2e+02 2e+02) (Variables|Default|GetDamping)) (.X (Math|Vector|BreakVector _scale)))
      (Rendering|Material|SetScalarParameterValue (Variables|Default|GetIntensity) "Intensity" (* (Math|Float|Clamp(Float) (Utilities|Array|Get(acopy) AudioValues (Variables|Default|GetMusicArrayIndex)) -2e+02 2e+02) (Variables|Default|GetGlowIntensity)) :!class /Script/Engine.MaterialInstanceDynamic :!label _label))
    (:NewEnumerator1
      (Variables|Default|SetMusicArrayIndex 1)
      (CallFunction|MoveZ _location_2 _location (/ (Math|Float|Clamp(Float) (Utilities|Array|Get(acopy) AudioValues (Variables|Default|GetMusicArrayIndex)) -2e+02 2e+02) (Variables|Default|GetDamping)) _z _rotation)
      (goto _label))
    (:NewEnumerator2
      (Variables|Default|SetMusicArrayIndex 2)
      (CallFunction|AggresiveAttack _location_2 (/ (Math|Float|Clamp(Float) (Utilities|Array|Get(acopy) AudioValues (Variables|Default|GetMusicArrayIndex)) -2e+02 2e+02) (Variables|Default|GetDamping)) _z)
      (goto _label))
    (:NewEnumerator3
      (Variables|Default|SetMusicArrayIndex 3))))

(fn MoveZ
  (params (ObjectVector :type Vector) (OldPosition :type Vector) (MusicValue :type Float%20%28single-precision%29) (MinimalZPos :type Float%20%28single-precision%29) (StartRotation :type Rotator))
  (bind _returnvalue (+ OldPosition (Math|Vector|MakeVector 0.0 0.0 0.0)))
  (Transformation|SetActorRelativeLocation (Math|Vector|MakeVector (.x _returnvalue) (.y _returnvalue) (Math|Float|Clamp(Float) (.z _returnvalue) -1e+02 5e+02))))

(fn ScaleonMusic
  (params (MusicValues :type Float%20%28single-precision%29) (MInimalScale :type Float%20%28single-precision%29))
  ;[1 1 1] scale
  (Transformation|SetActorScale3D (Math|Vector|ClampVectorSize (Math|Conversions|ToVector(Float) MusicValues) MInimalScale (Variables|Default|GetMaxScale))))

(fn AggresiveAttack
  (params (ObjectVector :type Vector) (MusicValues :type Float%20%28single-precision%29) (MinimalZPos :type Float%20%28single-precision%29))
  (bind (_x _y _z) (Math|Vector|BreakVector ObjectVector))
  (bind (_x_2 _y_2 _z_2) (Math|Vector|BreakVector ObjectVector))
  ;[1 1 1] Check if the music value is higher than minimal attack value.
  (if (>= MusicValues (Variables|Default|GetMinAggressionAttackValue))
    ;[1 1 1] Move Z attack
    (Transformation|SetActorLocation (Math|Vector|MakeVector _x_2 _y_2 (Math|Float|Clamp(Float) (+ _z_2 MusicValues) MinimalZPos 6e+02)) false false)
    (else
      ;[1 1 1] Move Z back to start positionZ
      (Transformation|SetActorLocation (Math|Vector|MakeVector _x _y (Math|Float|Lerp _z MinimalZPos 0.5)) false false))))