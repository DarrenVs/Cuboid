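; BP_Chunk is a scrolling world segment that a ChunkManager recycles.
; Each Tick moves it along negative X by Speed, without delta-time scaling, pinning Y and Z to zero.
; Once it passes two chunk lengths behind the origin, a DoOnce gate asks the manager to respawn it by ChunkID.
; The Respawned event resets that gate for the next pass.
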(event Custom|Respawned
  (Utilities|FlowControl|DoOnce false) ; enters at Reset
)

(event EventBeginPlay)

(event Collision|EventActorBeginOverlap
  (params (OtherActor :type Actor%20Object%20Reference)))

(event EventTick
  (params (DeltaSeconds :type Float%20%28single-precision%29))
  (bind _returnvalue (Transformation|GetActorLocation))
  (bind _chunkmanager (Variables|Default|GetChunkManager))
  (bind _x (Math|Vector|BreakVector _returnvalue))
  (bind _chunklength (Variables|/Game/Blueprints/BP_ChunkManager.BP_ChunkManager_C|GetChunkLength _chunkmanager))
  (if (< _x (Math|Conversions|ToFloat(Integer) (- (* _chunklength -1) _chunklength)))
    (Utilities|FlowControl|DoOnce false
      (:Completed
        (Default|RespawnChunk (Variables|Default|GetChunkManager) (Variables|Default|GetChunkID))))
    (else
      (Transformation|SetActorLocation (Math|Vector|MakeVector (- _x (Variables|Default|GetSpeed)) 0.0 0.0) false false))))

(fn ConstructionScript)