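; Grid-based chunk generator that lays out tiles as instanced static meshes and adds buildings when play starts.
; The construction script calls the parent's, then adds one instance per GridTiles entry, positioned on X and Y by TileSize.
; BeginPlay calls AddBuildings, whose logic is not defined in these graphs.
; An unconnected loop for doubling instance Z scale never runs, and Tick and overlap events are disabled.
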(event EventBeginPlay
  (|CallParentFunction)
  (CallFunction|AddBuildings 2))

(event Collision|EventActorBeginOverlap
  (params (OtherActor :type Actor%20Object%20Reference))
  (|CallParentFunction OtherActor) ; This node is disabled and will not be called.\nDrag off pins to build functionality.
)

(event EventTick
  (params (DeltaSeconds :type Float%20%28single-precision%29))
  (|CallParentFunction DeltaSeconds) ; This node is disabled and will not be called.\nDrag off pins to build functionality.
)

(fn ConstructionScript
  (bind _tilesize (Variables|Default|GetTileSize))
  (|CallParentFunction)
  (for _array_element (Variables|Default|GetGridTiles)
    (Components|InstancedStaticMesh|AddInstance (Variables|Default|GetInstancedStaticMesh) (Math|Transform|MakeTransform (Math|Vector|MakeVector (* (.X (Math|Vector2D|BreakVector2D _array_element)) _tilesize) (* (.Y (Math|Vector2D|BreakVector2D _array_element)) _tilesize) 0.0)))))