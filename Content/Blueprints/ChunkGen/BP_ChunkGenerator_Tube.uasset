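; Tube variant of the chunk generator that wraps a tile grid around the X axis and places buildings on it.
; The construction script lays instanced tiles in a ring, deriving each tile's position and roll from its grid Y.
; AddBuildings picks tiles for four building sizes, largest first, and each square footprint's averaged position and roll set the building transform.
; CreateBuildings spawns and attaches the actors, while GetBuilding only returns types and transforms.
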(event EventBeginPlay
  (|CallParentFunction))

(event Collision|EventActorBeginOverlap
  (params (OtherActor :type Actor%20Object%20Reference))
  (|CallParentFunction OtherActor) ; This node is disabled and will not be called.\nDrag off pins to build functionality.
)

(event EventTick
  (params (DeltaSeconds :type Float%20%28single-precision%29))
  (|CallParentFunction DeltaSeconds) ; This node is disabled and will not be called.\nDrag off pins to build functionality.
)

(fn ConstructionScript
  (|CallParentFunction)
  (Variables|Generation|SetGridAngle (/ 3.6e+02 (+ (.y (Variables|Default|GetGridSize)) 1.0)))
  (for _array_element (Variables|Default|GetGridTiles)
    (Components|InstancedStaticMesh|AddInstance (Variables|Default|GetInstancedStaticMesh) (Math|Transform|MakeTransform (Math|Vector|MakeVector (* (Variables|Generation|GetTileSize) (.x _array_element)) (.z (Math|Vector|RotateVectorAroundAxis (Math|Vector|MakeVector 0.0 (Variables|Generation|GetTubeSize) 0.0) (* (+ (.y _array_element) (/ (.y (Variables|Default|GetGridSize)) 2.0)) (Variables|Generation|GetGridAngle)) "5.000000,0.000000,0.000000")) (.y (Math|Vector|RotateVectorAroundAxis (Math|Vector|MakeVector 0.0 (Variables|Generation|GetTubeSize) 0.0) (* (+ (.y _array_element) (/ (.y (Variables|Default|GetGridSize)) 2.0)) (Variables|Generation|GetGridAngle)) "5.000000,0.000000,0.000000"))) (Math|Rotator|MakeRotator (+ (* (+ (.y _array_element) (/ (.y (Variables|Default|GetGridSize)) 2.0)) (Variables|Generation|GetGridAngle)) 1.8e+02) 0.0 0.0)))))

(fn PlaceBuildings
  (params (GridPositions :type Array%20of%20Integers) (BuildingType :type Integer))
  (bind _returnvalue (+ BuildingType 1))
  (bind _selectedrotations (LocalVariables|GetSelectedRotations))
  (bind (_arrayindex _arrayelement) (Utilities|Array|ReverseforEachLoop GridPositions)
    (:LoopBody
      (Utilities|Array|Add (LocalVariables|GetSelectedPositions) (Math|Vector|MakeVector (* (Variables|Generation|GetTileSize) (.x (Utilities|Array|Get(acopy) (Variables|Default|GetGridTiles) _arrayelement))) (.z (Math|Vector|RotateVectorAroundAxis (Math|Vector|MakeVector 0.0 (Variables|Generation|GetTubeSize) 0.0) (* (+ (.y (Utilities|Array|Get(acopy) (Variables|Default|GetGridTiles) _arrayelement)) (/ (.y (Variables|Default|GetGridSize)) 2.0)) (Variables|Generation|GetGridAngle)) "5.000000,0.000000,0.000000")) (.y (Math|Vector|RotateVectorAroundAxis (Math|Vector|MakeVector 0.0 (Variables|Generation|GetTubeSize) 0.0) (* (+ (.y (Utilities|Array|Get(acopy) (Variables|Default|GetGridTiles) _arrayelement)) (/ (.y (Variables|Default|GetGridSize)) 2.0)) (Variables|Generation|GetGridAngle)) "5.000000,0.000000,0.000000"))))
      (Utilities|Array|Add (LocalVariables|GetSelectedRotations) (+ (* (+ (.y (Utilities|Array|Get(acopy) (Variables|Default|GetGridTiles) _arrayelement)) (/ (.y (Variables|Default|GetGridSize)) 2.0)) (Variables|Generation|GetGridAngle)) 1.8e+02))
      (if (== (Math|Integer|%(Integer) _arrayindex (* _returnvalue _returnvalue)) 0)
        (for _array_element _selectedrotations
          (LocalVariables|SetAverageRotation (+ _array_element (LocalVariables|GetAverageRotation))))
        (bind _output_get (LocalVariables|SetAverageRotation (/ (LocalVariables|GetAverageRotation) (Math|Conversions|ToFloat(Integer) (Utilities|Array|Length _selectedrotations)))))
        (bind _returnvalue_2 (Game|SpawnActorfromClass "/Game/Blueprints/BuildingClass/BP_BuildingClass.BP_BuildingClass_C" (Math|Transform|MakeTransform (Math|Vector|GetVectorArrayAverage (LocalVariables|GetSelectedPositions)) (Math|Rotator|MakeRotator _output_get 0.0 0.0) "1,1,1") "Undefined" 0 (Utilities|Select :Index BuildingType :Option%200 "NewEnumerator0" :Option%201 "NewEnumerator1" :Option%202 "NewEnumerator2" :Option%203 "NewEnumerator3") (Utilities|Select :Index BuildingType :Option%200 "NewEnumerator0" :Option%201 "NewEnumerator0" :Option%202 "NewEnumerator1" :Option%203 "NewEnumerator1") 0))
        (Transformation|AttachActorToActor _returnvalue_2 self "None" "KeepRelative" "KeepRelative" "KeepRelative" true)
        (Utilities|Array|Add (Variables|Default|GetBuildings) _returnvalue_2)
        (Utilities|Array|Clear (LocalVariables|GetSelectedPositions))
        (Utilities|Array|Clear (LocalVariables|GetSelectedRotations))
        (LocalVariables|SetAverageRotation 0.0)))))

(fn ClearBuildings
  (for _array_element (Variables|Default|GetBuildings)
    (Actor|DestroyActor _array_element))
  (Utilities|Array|Clear (Variables|Default|GetBuildings))
  (Variables|Default|SetAvailableTiles (Variables|Default|GetGridTiles)))

(fn CreateBuildings
  (Utilities|FlowControl|Sequence
    (:then_0
      (bind _allcheckedfields (CallFunction|AddBuildings 3))
      (CallFunction|PlaceBuildings _allcheckedfields 3))
    (:then_1
      (bind _allcheckedfields_2 (CallFunction|AddBuildings 2))
      (CallFunction|PlaceBuildings _allcheckedfields_2 2))
    (:then_2
      (bind _allcheckedfields_3 (CallFunction|AddBuildings 1))
      (CallFunction|PlaceBuildings _allcheckedfields_3 1))
    (:then_3
      (bind _allcheckedfields_4 (CallFunction|AddBuildings))
      (CallFunction|PlaceBuildings _allcheckedfields_4))))

(fn GetBuilding
  (Utilities|FlowControl|Sequence
    (:then_0
      (Utilities|Array|Clear (LocalVariables|GetBuildingClasses))
      (Utilities|Array|Clear (LocalVariables|GetBuildingTransforms)))
    (:then_1
      (bind _allcheckedfields (CallFunction|AddBuildings 3))
      (bind (_buildingclass _transform) (CallFunction|GetBuildingPlacement _allcheckedfields 3))
      (Utilities|Array|AppendArray (LocalVariables|GetBuildingClasses) _buildingclass)
      (Utilities|Array|AppendArray (LocalVariables|GetBuildingTransforms) _transform))
    (:then_2
      (bind _allcheckedfields_2 (CallFunction|AddBuildings 2))
      (bind (_buildingclass_2 _transform_2) (CallFunction|GetBuildingPlacement _allcheckedfields_2 2))
      (Utilities|Array|AppendArray (LocalVariables|GetBuildingClasses) _buildingclass_2)
      (Utilities|Array|AppendArray (LocalVariables|GetBuildingTransforms) _transform_2))
    (:then_3
      (bind _allcheckedfields_3 (CallFunction|AddBuildings 1))
      (bind (_buildingclass_3 _transform_3) (CallFunction|GetBuildingPlacement _allcheckedfields_3 1))
      (Utilities|Array|AppendArray (LocalVariables|GetBuildingClasses) _buildingclass_3)
      (Utilities|Array|AppendArray (LocalVariables|GetBuildingTransforms) _transform_3))
    (:then_4
      (bind _allcheckedfields_4 (CallFunction|AddBuildings))
      (bind (_buildingclass_4 _transform_4) (CallFunction|GetBuildingPlacement _allcheckedfields_4))
      (Utilities|Array|AppendArray (LocalVariables|GetBuildingClasses) _buildingclass_4)
      (Utilities|Array|AppendArray (LocalVariables|GetBuildingTransforms) _transform_4))
    (:then_5
      (return (LocalVariables|GetBuildingClasses) (LocalVariables|GetBuildingTransforms)))))

(fn GetBuildingPlacement
  (params (GridPositions :type Array%20of%20Integers) (BuildingType :type Integer))
  (bind _returnvalue (+ BuildingType 1))
  (bind _selectedrotations (LocalVariables|GetSelectedRotations))
  (Utilities|Array|Clear (LocalVariables|GetBuildingClasses))
  (Utilities|Array|Clear (LocalVariables|GetTransforms))
  (bind (_arrayindex _arrayelement) (Utilities|Array|ReverseforEachLoop GridPositions)
    (:LoopBody
      (Utilities|Array|Add (LocalVariables|GetSelectedPositions) (Math|Vector|MakeVector (* (Variables|Generation|GetTileSize) (.x (Utilities|Array|Get(acopy) (Variables|Default|GetGridTiles) _arrayelement))) (.z (Math|Vector|RotateVectorAroundAxis (Math|Vector|MakeVector 0.0 (Variables|Generation|GetTubeSize) 0.0) (* (+ (.y (Utilities|Array|Get(acopy) (Variables|Default|GetGridTiles) _arrayelement)) (/ (.y (Variables|Default|GetGridSize)) 2.0)) (Variables|Generation|GetGridAngle)) "5.000000,0.000000,0.000000")) (.y (Math|Vector|RotateVectorAroundAxis (Math|Vector|MakeVector 0.0 (Variables|Generation|GetTubeSize) 0.0) (* (+ (.y (Utilities|Array|Get(acopy) (Variables|Default|GetGridTiles) _arrayelement)) (/ (.y (Variables|Default|GetGridSize)) 2.0)) (Variables|Generation|GetGridAngle)) "5.000000,0.000000,0.000000"))))
      (Utilities|Array|Add (LocalVariables|GetSelectedRotations) (+ (* (+ (.y (Utilities|Array|Get(acopy) (Variables|Default|GetGridTiles) _arrayelement)) (/ (.y (Variables|Default|GetGridSize)) 2.0)) (Variables|Generation|GetGridAngle)) 1.8e+02))
      (if (== (Math|Integer|%(Integer) _arrayindex (* _returnvalue _returnvalue)) 0)
        (for _array_element _selectedrotations
          (LocalVariables|SetAverageRotation (+ _array_element (LocalVariables|GetAverageRotation))))
        (bind _output_get (LocalVariables|SetAverageRotation (/ (LocalVariables|GetAverageRotation) (Math|Conversions|ToFloat(Integer) (Utilities|Array|Length _selectedrotations)))))
        (Utilities|Array|Add (LocalVariables|GetBuildingClasses) (Utilities|Select :Index BuildingType :Option%200 "NewEnumerator0" :Option%201 "NewEnumerator1" :Option%202 "NewEnumerator2" :Option%203 "NewEnumerator3"))
        (Utilities|Array|Add (LocalVariables|GetTransforms) (Math|Transform|MakeTransform (Math|Vector|GetVectorArrayAverage (LocalVariables|GetSelectedPositions)) (Math|Rotator|MakeRotator _output_get 0.0 0.0) "1.000000,1,1"))
        (Utilities|Array|Clear (LocalVariables|GetSelectedPositions))
        (Utilities|Array|Clear (LocalVariables|GetSelectedRotations))
        (LocalVariables|SetAverageRotation 0.0)))
    (:Completed
      (return (LocalVariables|GetBuildingClasses) (LocalVariables|GetTransforms)))))