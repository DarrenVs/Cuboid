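; Chunk generator that builds a centred 2D tile grid in its construction script and provides random placement of four building sizes on it.
; AddBuildings picks random available tiles for square footprints from 1x1 to 4x4, retrying up to a limit.
; CheckFieldEmpty validates each footprint, then removes it and border tiles from SelectSurroundingFields from the available pool to space buildings.
; Chosen tiles are returned and shown as height-scaled debug mesh instances; nothing here calls AddBuildings.
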(event EventBeginPlay)

(event Collision|EventActorBeginOverlap
  (params (OtherActor :type Actor%20Object%20Reference)))

(event EventTick
  (params (DeltaSeconds :type Float%20%28single-precision%29)))

(fn ConstructionScript
  ;[1 1 1] Create a new empty grid
  (Utilities|Array|Clear (Variables|GridSettings|GetGridTiles))
  (CallFunction|CreateGrid))

(fn CreateGrid
  (bind _gridsize (Variables|GridSettings|GetGridSize))
  (bind _gridsize_2 (Variables|GridSettings|GetGridSize))
  (Utilities|FlowControl|Sequence
    (:then_0
      ;[1 1 1] Create grid of specified size
      (for _index (range 0 (Math|Float|Truncate (.x _gridsize)))
        (for _index_2 (range 0 (Math|Float|Truncate (.y _gridsize)))
          (Utilities|Array|Add (Variables|GridSettings|GetGridTiles) (Math|Vector2D|MakeVector2D (Math|Conversions|ToFloat(Integer) _index) (Math|Conversions|ToFloat(Integer) _index_2))))))
    (:then_1
      ;[1 1 1] Center grid & tiles
      (for (_array_element _array_index) (Variables|GridSettings|GetGridTiles)
        (Utilities|Array|SetArrayElem (Variables|GridSettings|GetGridTiles) _array_index (Math|Vector2D|MakeVector2D (- (.X (Math|Vector2D|BreakVector2D _array_element)) (/ (.x _gridsize_2) 2.0)) (- (.Y (Math|Vector2D|BreakVector2D _array_element)) (/ (.y _gridsize_2) 2.0))))))
    (:then_2
      ;[1 1 1] Make all tiles available tiles
      (Variables|GridSettings|SetAvailableTiles (Variables|GridSettings|GetGridTiles)))))

(fn AddBuildings
  (params (BuildingType :type Integer))
  (bind _instancedstaticmesh (Variables|Default|GetInstancedStaticMesh))
  (bind _instancedstaticmesh_2 (Variables|Default|GetInstancedStaticMesh))
  (bind _instancedstaticmesh_3 (Variables|Default|GetInstancedStaticMesh))
  (bind _instancedstaticmesh_4 (Variables|Default|GetInstancedStaticMesh))
  (bind _allreturnfields (LocalVariables|GetAllReturnFields))
  (LocalVariables|SetBuildingPlaceTries 0) ; Reset pogingen
  (Utilities|FlowControl|ForLoopwithBreak 1 (Utilities|Select :Index BuildingType :Option%200 (Variables|GridSettings|GetMaxBuildingsA) :Option%201 (Variables|GridSettings|GetMaxBuildingsB) :Option%202 (Variables|GridSettings|GetMaxBuildingsC) :Option%203 (Variables|GridSettings|GetMaxBuildingsD)) :!label _label ; Loop door de benodigde gebouwen heen
    (:LoopBody
      (LocalVariables|SetCurrentTile (Math|Random|RandomInteger (Utilities|Array|Length (Variables|GridSettings|GetAvailableTiles))) :!label _label_2)
      (switch int BuildingType ; Switch building class
        (:0
          ;[1 1 1] Check lege velden
          (bind (_arefieldsempty _allcheckedfields) (CallFunction|CheckFieldEmpty (LocalVariables|GetCurrentTile) 1))
          (if _arefieldsempty
            ;[1 1 1] Loop door de lege velden
            (for _array_element _allcheckedfields
              ;[1 0.02665 0] Update de debug velden om gekozen velden te visualizeren
              (Components|InstancedStaticMesh|UpdateInstanceTransform _instancedstaticmesh_2 _array_element (Math|Transform|MakeTransform (.Location (Math|Transform|BreakTransform (.OutInstanceTransform (Components|InstancedStaticMesh|GetInstanceTransform _instancedstaticmesh_2 _array_element false)))) (.Rotation (Math|Transform|BreakTransform (.OutInstanceTransform (Components|InstancedStaticMesh|GetInstanceTransform _instancedstaticmesh_2 _array_element false)))) "1,1,1.500000") false true false)
              ;[1 1 1] Onthoud gekozen velden
              (Utilities|Array|Add _allreturnfields _array_element))
            (else
              (if (>= (LocalVariables|GetBuildingPlaceTries) (Variables|GridSettings|GetMaxBuildingPlacementTries)) :!label _label_3 ; Retry if couldn't place the first time
                (goto _label Break)
                (else
                  (Math|Integer|IncrementInt (LocalVariables|GetBuildingPlaceTries) ; Retry
                    (:%20%20
                      (goto _label_2))))))))
        (:1
          (bind (_arefieldsempty_2 _allcheckedfields_2) (CallFunction|CheckFieldEmpty (LocalVariables|GetCurrentTile) 2))
          (if _arefieldsempty_2
            (for _array_element_2 _allcheckedfields_2
              (Components|InstancedStaticMesh|UpdateInstanceTransform _instancedstaticmesh_3 _array_element_2 (Math|Transform|MakeTransform (.Location (Math|Transform|BreakTransform (.OutInstanceTransform (Components|InstancedStaticMesh|GetInstanceTransform _instancedstaticmesh_3 _array_element_2 false)))) (.Rotation (Math|Transform|BreakTransform (.OutInstanceTransform (Components|InstancedStaticMesh|GetInstanceTransform _instancedstaticmesh_3 _array_element_2 false)))) "1,1,2.000000") false true false)
              (Utilities|Array|Add _allreturnfields _array_element_2))
            (else
              (goto _label_3))))
        (:2
          (bind (_arefieldsempty_3 _allcheckedfields_3) (CallFunction|CheckFieldEmpty (LocalVariables|GetCurrentTile) 3))
          (if _arefieldsempty_3
            (for _array_element_3 _allcheckedfields_3
              (Components|InstancedStaticMesh|UpdateInstanceTransform _instancedstaticmesh_4 _array_element_3 (Math|Transform|MakeTransform (.Location (Math|Transform|BreakTransform (.OutInstanceTransform (Components|InstancedStaticMesh|GetInstanceTransform _instancedstaticmesh_4 _array_element_3 false)))) (.Rotation (Math|Transform|BreakTransform (.OutInstanceTransform (Components|InstancedStaticMesh|GetInstanceTransform _instancedstaticmesh_4 _array_element_3 false)))) "1,1,3.000000") false true false)
              (Utilities|Array|Add _allreturnfields _array_element_3))
            (else
              (goto _label_3))))
        (:3
          (bind (_arefieldsempty_4 _allcheckedfields_4) (CallFunction|CheckFieldEmpty (LocalVariables|GetCurrentTile) 4))
          (if _arefieldsempty_4
            (for _array_element_4 _allcheckedfields_4
              (Components|InstancedStaticMesh|UpdateInstanceTransform _instancedstaticmesh _array_element_4 (Math|Transform|MakeTransform (.Location (Math|Transform|BreakTransform (.OutInstanceTransform (Components|InstancedStaticMesh|GetInstanceTransform _instancedstaticmesh _array_element_4 false)))) (.Rotation (Math|Transform|BreakTransform (.OutInstanceTransform (Components|InstancedStaticMesh|GetInstanceTransform _instancedstaticmesh _array_element_4 false)))) "1,1,3.000000") false true false)
              (Utilities|Array|Add _allreturnfields _array_element_4))
            (else
              (goto _label_3))))))
    (:Completed
      ;[1 1 1] Return values
      (return (LocalVariables|GetAllReturnFields)))))

(fn CheckFieldEmpty
  (params (CornerTile :type Integer) (FieldSize :type Integer))
  (bind _returnvalue (- FieldSize 1))
  ;[1 1 1] Reset voor de check
  (LocalVariables|SetHasFoundMatchingField false)
  (Utilities|Array|Clear (LocalVariables|GetCheckedFields))
  (for _index (range 0 _returnvalue) ; Y-axis fields
    (for _index_2 (range 0 _returnvalue) ; X-axis fields
      (bind _array_element (Utilities|Array|ForEachLoopwithBreak (Variables|GridSettings|GetAvailableTiles) :!label _label)
        (:LoopBody
          (bind _output_get (LocalVariables|SetHasFoundMatchingField (Math|Vector|Equal(Vector) (+ (Utilities|Array|Get(acopy) (Variables|GridSettings|GetAvailableTiles) CornerTile) (Math|Vector2D|MakeVector2D (Math|Conversions|ToFloat(Integer) _index_2) (Math|Conversions|ToFloat(Integer) _index))) _array_element 0.1))) ; Set boolean
          (if _output_get ; If matching field has been found
            (Utilities|Array|Add (LocalVariables|GetCheckedFields) (Utilities|Array|FindItem (Variables|GridSettings|GetGridTiles) (+ (Utilities|Array|Get(acopy) (Variables|GridSettings|GetAvailableTiles) CornerTile) (Math|Vector2D|MakeVector2D (Math|Conversions|ToFloat(Integer) _index_2) (Math|Conversions|ToFloat(Integer) _index))))) ; Add found tile to array
            (goto _label Break)))
        (:Completed
          (if (not (LocalVariables|GetHasFoundMatchingField)) ; Check for found fields when finished
            (return false 0) ; Return false if fields not empty
          )))))
  (Utilities|FlowControl|Sequence
    (:then_0
      (bind _surroundingfieldcoordinates (CallFunction|SelectSurroundingFields (LocalVariables|GetCheckedFields))) ; Remove surrounding fields to prevent clipping
      (for _array_element_2 _surroundingfieldcoordinates ; Loop through found fields
        (Utilities|Array|RemoveItem (Variables|GridSettings|GetAvailableTiles) _array_element_2)))
    (:then_1
      (if (> (Utilities|Array|Length (LocalVariables|GetCheckedFields)) (* FieldSize FieldSize))
        (Utilities|RemoveDoublesfromArray (LocalVariables|GetCheckedFields)) ; Remove duplicate field entries from array
      ))
    (:then_2
      (for _array_element_3 (LocalVariables|GetCheckedFields) ; Remove from available fields
        (Utilities|Array|RemoveItem (Variables|GridSettings|GetAvailableTiles) (Utilities|Array|Get(acopy) (Variables|GridSettings|GetGridTiles) _array_element_3)) ; Remove all selected tiles from available tiles
      )
      (return true (LocalVariables|GetCheckedFields)) ; Field is empty
    )))

(fn SelectSurroundingFields
  (params (CurrentFields :type Array%20of%20Integers))
  (Utilities|FlowControl|Sequence
    (:then_0
      (bind _output_get (LocalVariables|SetSmallestVector (Utilities|Array|Get(acopy) (Variables|GridSettings|GetGridTiles) (Utilities|Array|Get(acopy) CurrentFields)))) ; Set field smallest X/Y
      (LocalVariables|SetLargestVector _output_get) ; Set field largest X/Y
    )
    (:then_1
      ;[1 1 1] Set largest field X & Y
      (for _array_element CurrentFields
        (Utilities|FlowControl|Sequence
          (:then_0
            (if (> (.x (Utilities|Array|Get(acopy) (Variables|GridSettings|GetGridTiles) _array_element)) (.x (LocalVariables|GetLargestVector)))
              (LocalVariables|SetLargestVector (Math|Vector2D|MakeVector2D (.x (Utilities|Array|Get(acopy) (Variables|GridSettings|GetGridTiles) _array_element)) (.y (LocalVariables|GetLargestVector))))
              (Math|Integer|IncrementInt (LocalVariables|GetAmountOfFieldsX))))
          (:then_1
            (if (> (.y (Utilities|Array|Get(acopy) (Variables|GridSettings|GetGridTiles) _array_element)) (.y (LocalVariables|GetLargestVector)))
              (LocalVariables|SetLargestVector (Math|Vector2D|MakeVector2D (.x (LocalVariables|GetLargestVector)) (.y (Utilities|Array|Get(acopy) (Variables|GridSettings|GetGridTiles) _array_element))))
              (Math|Integer|IncrementInt (LocalVariables|GetAmountOfFieldsY)))))))
    (:then_2
      (for _index (range 0 (LocalVariables|GetAmountOfFieldsX)) ; Add fields above
        (Utilities|Array|Add (LocalVariables|GetBorderFields) (Math|Vector2D|MakeVector2D (+ (Math|Conversions|ToFloat(Integer) _index) (.x (LocalVariables|GetSmallestVector))) (- (.y (LocalVariables|GetSmallestVector)) 1.0)))))
    (:then_3
      (for _index_2 (range 0 (LocalVariables|GetAmountOfFieldsY)) ; Add fields to the left
        (Utilities|Array|Add (LocalVariables|GetBorderFields) (Math|Vector2D|MakeVector2D (- (.x (LocalVariables|GetSmallestVector)) 1.0) (+ (Math|Conversions|ToFloat(Integer) _index_2) (.y (LocalVariables|GetSmallestVector)))))))
    (:then_4
      (for _index_3 (range 0 (LocalVariables|GetAmountOfFieldsX)) ; Add fields below
        (Utilities|Array|Add (LocalVariables|GetBorderFields) (Math|Vector2D|MakeVector2D (- (.x (LocalVariables|GetLargestVector)) (Math|Conversions|ToFloat(Integer) _index_3)) (+ (.y (LocalVariables|GetLargestVector)) 1.0)))))
    (:then_5
      (for _index_4 (range 0 (LocalVariables|GetAmountOfFieldsY)) ; Add fields to the right
        (Utilities|Array|Add (LocalVariables|GetBorderFields) (Math|Vector2D|MakeVector2D (+ (.x (LocalVariables|GetSmallestVector)) 1.0) (- (.y (LocalVariables|GetSmallestVector)) (Math|Conversions|ToFloat(Integer) _index_4))))))
    (:then_6
      (return (LocalVariables|GetBorderFields)) ; Return all bordering fields
    )))