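; Tube chunk generator variant that scrolls toward negative X and recycles itself with instanced buildings.
; BeginPlay spawns a BP_InstancedBuildings actor and attaches it to the chunk.
; Tick moves the chunk by Speed each frame until it falls two chunk lengths behind the origin.
; A DoOnce, re-armed by Respawn, then has ChunkManager respawn the chunk, clears the buildings and places a fresh GetBuilding layout.
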(event Custom|Respawn
  (bind _buildinginstance (Variables|Default|GetBuildingInstance))
  (Variables|Default|SetAvailableTiles (Variables|Default|GetGridTiles))
  (Utilities|FlowControl|DoOnce false) ; enters at Reset
)

(event EventBeginPlay
  (|CallParentFunction)
  (bind _returnvalue (Game|SpawnActorfromClass "/Game/Blueprints/ChunkGen/BP_InstancedBuildings.BP_InstancedBuildings_C" (Math|Transform|MakeTransform "3300.000000, 0, 0") "Undefined" 0 0))
  (bind _output_get (Variables|Default|SetBuildingInstance _returnvalue))
  (Transformation|AttachActorToActor _output_get self "None" "KeepRelative" "KeepRelative" "KeepRelative" true))

(event Collision|EventActorBeginOverlap
  (params (OtherActor :type Actor%20Object%20Reference))
  (|CallParentFunction OtherActor) ; This node is disabled and will not be called.\nDrag off pins to build functionality.
)

(event EventTick
  (params (DeltaSeconds :type Float%20%28single-precision%29))
  (bind _returnvalue (Transformation|GetActorLocation))
  (bind _chunkmanager (Variables|Default|GetChunkManager))
  (bind _buildinginstance (Variables|Default|GetBuildingInstance))
  (bind _x (Math|Vector|BreakVector _returnvalue))
  (bind _chunklength (Variables|/Game/Blueprints/BP_ChunkManager.BP_ChunkManager_C|GetChunkLength _chunkmanager))
  (|CallParentFunction DeltaSeconds)
  (if (< _x (Math|Conversions|ToFloat(Integer) (- (* _chunklength -1) _chunklength)))
    (Utilities|FlowControl|DoOnce false
      (:Completed
        (Default|RespawnChunk (Variables|Default|GetChunkManager) (Variables|Default|GetChunkID))
        (Default|ClearBuildings _buildinginstance)
        (bind (_buildingclass _transform) (CallFunction|GetBuilding))
        (for (_array_element _array_index) _buildingclass
          (Default|PlaceBuilding _buildinginstance _array_element (Utilities|Array|Get(acopy) _transform _array_index)))))
    (else
      (Transformation|SetActorLocation (Math|Vector|MakeVector (- _x (Variables|Default|GetSpeed)) 0.0 0.0) false false))))

(fn ConstructionScript
  (|CallParentFunction))

(fn PlaceInstancedBuildings)