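; Audio manager Blueprint that plays a random song and drives music-reactive object movement through InteractiveManager.
; The construction script picks a track from AudioFiles, sets it on the Audio component and starts playback.
; Each Tick samples a five-band frequency spectrum of that track, timed by game time plus a small look-ahead, and passes it to MoveObjects.
; GatherAllInteractionObjects is an empty stub.
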(event EventBeginPlay)

(event Collision|EventActorBeginOverlap
  (params (OtherActor :type Actor%20Object%20Reference)))

(event EventTick
  (params (DeltaSeconds :type Float%20%28single-precision%29))
  (bind _frequencyspectrum (CallFunction|CalculateAudioVisualization 5))
  (Default|MoveObjects (Variables|Default|GetInteractiveManager) _frequencyspectrum))

(fn ConstructionScript
  (CallFunction|PlayNewSong))

(fn CalculateAudioVisualization
  (params (AmountOfChannels :type Integer))
  (bind _outspectrum (Class|SoundVisualizationStatics|CalculateFrequencySpectrum (Utilities|Array|Get(acopy) (Variables|Default|GetAudioFiles) (Variables|Default|GetCurrentSong)) 0 (+ (Utilities|Time|GetGameTimeinSeconds) 0.08) 0.19 AmountOfChannels))
  (bind _output_get (Variables|Default|SetAudioVariables _outspectrum))
  (return _output_get))

(fn PlayNewSong
  (bind _audiofiles (Variables|Default|GetAudioFiles))
  (bind _audio (Variables|Default|GetAudio))
  (bind _output_get (Variables|Default|SetCurrentSong (Math|Random|RandomIntegerinRange 0 (Utilities|Array|Length _audiofiles))))
  (Audio|Components|Audio|SetSound _audio (Utilities|Array|Get(acopy) _audiofiles _output_get))
  (Audio|Components|Audio|Play _audio 0.0))

(fn GatherAllInteractionObjects)