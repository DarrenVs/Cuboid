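; BP_Billboards is a floating score display that follows a referenced actor and turns to face the player camera.
; Each tick it eases toward the MovePosition actor plus an offset using a fixed-alpha lerp, which depends on frame rate.
; Its rotation comes from the flattened direction to the camera, so it stays upright.
; The Score text shows a test value that accumulates elapsed time, standing in for a real score.
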(event EventTick
  (params (DeltaSeconds :type Float%20%28single-precision%29))
  (bind _output_get (Variables|Default|SetTestScoreValue (+ (Variables|Default|GetTestScoreValue) DeltaSeconds)))
  (Rendering|Components|TextRender|SetText (Variables|Default|GetScore) (Utilities|Text|ToText(Float) _output_get "HalfToEven"))
  (Transformation|SetActorTransform (Math|Transform|MakeTransform (Math|Vector|Lerp(Vector) (Transformation|GetActorLocation) (+ (Transformation|GetActorLocation (Variables|Default|GetMovePosition)) (Variables|Default|GetOffsetFollow)) 0.2) (Math|Conversions|RotationFromXVector (Math|Vector|RotateVector (Math|Vector|Normalize (* (- (Transformation|GetActorLocation (Game|GetPlayerCameraManager 0)) (Transformation|GetActorLocation)) "1.000000,1.000000,0.000000")) "0, 0, 0")))))

(fn ConstructionScript)