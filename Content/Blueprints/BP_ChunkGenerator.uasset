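; Procedural chunk generator that lays out a centered tile grid and randomly places three sizes of placeholder buildings on it.
; The construction script builds the grid as instanced static meshes, and BeginPlay places buildings from largest to smallest.
; CheckFieldEmpty tests square footprints against available tiles with limited retries, and claimed tiles get taller Z scales.
; SelectSurroundingFields computes border tiles for spacing, but its call is disconnected.
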(event EventBeginPlay
  (CallFunction|AddBuildings 2)
  (CallFunction|AddBuildings 1)
  (CallFunction|AddBuildings))

(event Collision|EventActorBeginOverlap
  (params (OtherActor :type Actor%20Object%20Reference)))

(event EventTick
  (params (DeltaSeconds :type Float%20%28single-precision%29)))

(fn ConstructionScript
  (Utilities|Array|Clear (Variables|Default|GetGridTiles))
  (CallFunction|CreateGrid))

(fn CreateGrid
  (bind _gridsize (Variables|Default|GetGridSize))
  (bind _fieldsize (Variables|Default|GetFieldSize))
  (bind _gridsize_2 (Variables|Default|GetGridSize))
  (Utilities|FlowControl|Sequence
    (:then_0
      ;[1 1 1] Create grid of specified size
      (for _index (range 0 (Math|Float|Truncate (.x _gridsize)))
        (for _index_2 (range 0 (Math|Float|Truncate (.y _gridsize)))
          (Utilities|Array|Add (Variables|Default|GetGridTiles) (Math|Vector2D|MakeVector2D (* _index (Variables|Default|GetFieldSize)) (* _index_2 (Variables|Default|GetFieldSize)))))))
    (:then_1
      ;[1 1 1] Center grid & tiles
      (for (_array_element _array_index) (Variables|Default|GetGridTiles)
        (Utilities|Array|SetArrayElem (Variables|Default|GetGridTiles) _array_index (Math|Vector2D|MakeVector2D (- (.X (Math|Vector2D|BreakVector2D _array_element)) (/ (* (.x _gridsize_2) _fieldsize) 2.0)) (- (.Y (Math|Vector2D|BreakVector2D _array_element)) (/ (* (.y _gridsize_2) _fieldsize) 2.0))))))
    (:then_2
      ;[1 0 0.0758] Add instances to the grid (TEMP - FOR VISUALIZATION)
      (for _array_element_2 (Variables|Default|GetGridTiles)
        (Components|InstancedStaticMesh|AddInstance (Variables|Default|GetInstancedStaticMesh) (Math|Transform|MakeTransform (Math|Vector|MakeVector (.X (Math|Vector2D|BreakVector2D _array_element_2)) (.Y (Math|Vector2D|BreakVector2D _array_element_2)) 0.0)))))
    (:then_3
      ;[1 1 1] Make all tiles available tiles
      (Variables|Default|SetAvailableTiles (Variables|Default|GetGridTiles)))))

(fn AddBuildings
  (params (BuildingType :type Integer))
  (bind _instancedstaticmesh (Variables|Default|GetInstancedStaticMesh))
  (bind _instancedstaticmesh_2 (Variables|Default|GetInstancedStaticMesh))
  (bind _instancedstaticmesh_3 (Variables|Default|GetInstancedStaticMesh))
  (LocalVariables|SetBuildingPlaceTries 0)
  (Utilities|FlowControl|ForLoopwithBreak 1 (Utilities|Select :Index BuildingType :Option%200 (Variables|Default|GetMaxBuildingsA) :Option%201 (Variables|Default|GetMaxBuildingsB) :Option%202 (Variables|Default|GetMaxBuildingsC)) :!label _label
    (:LoopBody
      (LocalVariables|SetCurrentTile (Math|Random|RandomInteger (Utilities|Array|Length (Variables|Default|GetAvailableTiles))) :!label _label_2)
      (switch int BuildingType
        (:0
          (bind (_arefieldsempty _allcheckedfields) (CallFunction|CheckFieldEmpty (LocalVariables|GetCurrentTile) 1))
          (if _arefieldsempty
            (for _array_element _allcheckedfields
              (Components|InstancedStaticMesh|UpdateInstanceTransform _instancedstaticmesh_2 _array_element (Math|Transform|MakeTransform (.Location (Math|Transform|BreakTransform (.OutInstanceTransform (Components|InstancedStaticMesh|GetInstanceTransform _instancedstaticmesh_2 _array_element false)))) (.Rotation (Math|Transform|BreakTransform (.OutInstanceTransform (Components|InstancedStaticMesh|GetInstanceTransform _instancedstaticmesh_2 _array_element false)))) "1,1,1.500000") false true false))
            (else
              (if (>= (LocalVariables|GetBuildingPlaceTries) (Variables|Default|GetMaxBuildingPlacementTries)) :!label _label_3 ; Retry if couldn't place the first time
                (goto _label Break)
                (else
                  (Math|Integer|IncrementInt (LocalVariables|GetBuildingPlaceTries)
                    (:%20%20
                      (goto _label_2))))))))
        (:1
          (bind (_arefieldsempty_2 _allcheckedfields_2) (CallFunction|CheckFieldEmpty (LocalVariables|GetCurrentTile) 2))
          (if _arefieldsempty_2
            (for _array_element_2 _allcheckedfields_2
              (Components|InstancedStaticMesh|UpdateInstanceTransform _instancedstaticmesh_3 _array_element_2 (Math|Transform|MakeTransform (.Location (Math|Transform|BreakTransform (.OutInstanceTransform (Components|InstancedStaticMesh|GetInstanceTransform _instancedstaticmesh_3 _array_element_2 false)))) (.Rotation (Math|Transform|BreakTransform (.OutInstanceTransform (Components|InstancedStaticMesh|GetInstanceTransform _instancedstaticmesh_3 _array_element_2 false)))) "1,1,2.000000") false true false))
            (else
              (goto _label_3))))
        (:2
          (bind (_arefieldsempty_3 _allcheckedfields_3) (CallFunction|CheckFieldEmpty (LocalVariables|GetCurrentTile) 3))
          (if _arefieldsempty_3
            (for _array_element_3 _allcheckedfields_3
              (Components|InstancedStaticMesh|UpdateInstanceTransform _instancedstaticmesh _array_element_3 (Math|Transform|MakeTransform (.Location (Math|Transform|BreakTransform (.OutInstanceTransform (Components|InstancedStaticMesh|GetInstanceTransform _instancedstaticmesh _array_element_3 false)))) (.Rotation (Math|Transform|BreakTransform (.OutInstanceTransform (Components|InstancedStaticMesh|GetInstanceTransform _instancedstaticmesh _array_element_3 false)))) "1,1,3.000000") false true false))
            (else
              (goto _label_3))))))))

(fn CheckFieldEmpty
  (params (CornerTile :type Integer) (FieldSize :type Integer))
  (bind _returnvalue (- FieldSize 1))
  (LocalVariables|SetHasFoundMatchingField false)
  (Utilities|Array|Clear (LocalVariables|GetCheckedFields))
  (for _index (range 0 _returnvalue) ; Y-axis fields
    (for _index_2 (range 0 _returnvalue) ; X-axis fields
      (bind _array_element (Utilities|Array|ForEachLoopwithBreak (Variables|Default|GetAvailableTiles) :!label _label) ; Loop through available tiles to compare
        (:LoopBody
          (bind _output_get (LocalVariables|SetHasFoundMatchingField (Math|Vector|Equal(Vector) (+ (Utilities|Array|Get(acopy) (Variables|Default|GetAvailableTiles) CornerTile) (Math|Vector2D|MakeVector2D (* _index_2 (Variables|Default|GetFieldSize)) (* _index (Variables|Default|GetFieldSize)))) _array_element 1.0)))
          (if _output_get ; If matching field has been found
            (goto _label Break)
            (else
              (Utilities|Array|Add (LocalVariables|GetCheckedFields) (Utilities|Array|FindItem (Variables|Default|GetGridTiles) (+ (Utilities|Array|Get(acopy) (Variables|Default|GetAvailableTiles) CornerTile) (Math|Vector2D|MakeVector2D (* _index_2 (Variables|Default|GetFieldSize)) (* _index (Variables|Default|GetFieldSize)))))))))
        (:Completed
          (if (not (LocalVariables|GetHasFoundMatchingField))
            (return false 0))))))
  (Utilities|FlowControl|Sequence
    (:then_1
      (for _array_element_2 (LocalVariables|GetCheckedFields) ; Remove from available fields
        (Utilities|Array|RemoveItem (Variables|Default|GetAvailableTiles) (Utilities|Array|Get(acopy) (Variables|Default|GetGridTiles) _array_element_2)))
      (return true (LocalVariables|GetCheckedFields)) ; Field is empty
    )))

(fn SelectSurroundingFields
  (params (CurrentFields :type Array%20of%20Integers))
  (Utilities|FlowControl|Sequence
    (:then_0
      (for _array_element CurrentFields
        (Utilities|FlowControl|Sequence
          (:then_0
            (if (< (.x (Utilities|Array|Get(acopy) (Variables|Default|GetGridTiles) _array_element)) (.x (LocalVariables|GetSmallestVector)))
              (LocalVariables|SetSmallestVector (Math|Vector2D|MakeVector2D (.x (Utilities|Array|Get(acopy) (Variables|Default|GetGridTiles) _array_element)) (.y (LocalVariables|GetSmallestVector))))
              (Math|Integer|IncrementInt (LocalVariables|GetAmountOfFieldsX))))
          (:then_1
            (if (< (.y (Utilities|Array|Get(acopy) (Variables|Default|GetGridTiles) _array_element)) (.y (LocalVariables|GetSmallestVector)))
              (LocalVariables|SetSmallestVector (Math|Vector2D|MakeVector2D (.x (LocalVariables|GetSmallestVector)) (.y (Utilities|Array|Get(acopy) (Variables|Default|GetGridTiles) _array_element))))
              (Math|Integer|IncrementInt (LocalVariables|GetAmountOfFieldsY))))
          (:then_2
            (if (> (.x (Utilities|Array|Get(acopy) (Variables|Default|GetGridTiles) _array_element)) (.x (LocalVariables|GetLargestVector)))
              (LocalVariables|SetLargestVector (Math|Vector2D|MakeVector2D (.x (Utilities|Array|Get(acopy) (Variables|Default|GetGridTiles) _array_element)) (.y (LocalVariables|GetLargestVector))))
              (Math|Integer|IncrementInt (LocalVariables|GetAmountOfFieldsX))))
          (:then_3
            (if (> (.y (Utilities|Array|Get(acopy) (Variables|Default|GetGridTiles) _array_element)) (.y (LocalVariables|GetLargestVector)))
              (LocalVariables|SetLargestVector (Math|Vector2D|MakeVector2D (.x (LocalVariables|GetLargestVector)) (.y (Utilities|Array|Get(acopy) (Variables|Default|GetGridTiles) _array_element))))
              (Math|Integer|IncrementInt (LocalVariables|GetAmountOfFieldsY)))))))
    (:then_1
      (for _index (range 0 (LocalVariables|GetAmountOfFieldsX)) ; Add fields above
        (Utilities|Array|Add (LocalVariables|GetBorderFields) (Math|Vector2D|MakeVector2D (+ (* _index (Variables|Default|GetFieldSize)) (.x (LocalVariables|GetSmallestVector))) (- (.y (LocalVariables|GetSmallestVector)) (Variables|Default|GetFieldSize))))))
    (:then_2
      (for _index_2 (range 0 (LocalVariables|GetAmountOfFieldsY)) ; Add fields to the left
        (Utilities|Array|Add (LocalVariables|GetBorderFields) (Math|Vector2D|MakeVector2D (- (.x (LocalVariables|GetSmallestVector)) (Variables|Default|GetFieldSize)) (+ (* _index_2 (Variables|Default|GetFieldSize)) (.y (LocalVariables|GetSmallestVector)))))))
    (:then_3
      (for _index_3 (range 0 (LocalVariables|GetAmountOfFieldsX)) ; Add fields below
        (Utilities|Array|Add (LocalVariables|GetBorderFields) (Math|Vector2D|MakeVector2D (- (.x (LocalVariables|GetLargestVector)) (* _index_3 (Variables|Default|GetFieldSize))) (+ (.y (LocalVariables|GetLargestVector)) (Variables|Default|GetFieldSize))))))
    (:then_4
      (for _index_4 (range 0 (LocalVariables|GetAmountOfFieldsY)) ; Add fields to the right
        (Utilities|Array|Add (LocalVariables|GetBorderFields) (Math|Vector2D|MakeVector2D (+ (.x (LocalVariables|GetSmallestVector)) (Variables|Default|GetFieldSize)) (- (.y (LocalVariables|GetSmallestVector)) (* _index_4 (Variables|Default|GetFieldSize)))))))
    (:then_5
      (return (LocalVariables|GetBorderFields)))))