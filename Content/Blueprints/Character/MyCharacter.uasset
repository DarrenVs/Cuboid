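; Character Blueprint prototyping a health and shield damage system, with debug text for invincibility, health and shield.
; TakeDamage honours invincibility and shield unless bypassed, and damage events add timed invincibility or knockout.
; Get/Set helpers scale values by multipliers and clamp stored ones, though SetShield divides by HealthMultiplier rather than ShieldMultiplier.
; BeginPlay endlessly fires shield-ignoring damage after short delays, apparently as a test.
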(event Custom|Any%20Damage_Event
  (params (Damage :type Float%20%28single-precision%29) (Ignore%20Shield :type Boolean) (Ignore%20Invincible :type Boolean) (Damage%20Cooldown :type Float%20%28single-precision%29))
  (CallFunction|TakeDamage Damage Ignore%20Shield Ignore%20Invincible)
  (Variables|Default|SetInvincible true)
  (Utilities|FlowControl|Delay Damage%20Cooldown)
  (Variables|Default|SetInvincible false))

(event Custom|Knockback%20Damage_Event
  (params (Damage :type Float%20%28single-precision%29) (Ignore%20Shield :type Boolean) (Ignore%20Invincible :type Boolean) (Knockout%20Duration :type Float%20%28single-precision%29))
  (CallFunction|TakeDamage Damage Ignore%20Shield Ignore%20Invincible)
  (Variables|Default|SetKnockedout true)
  (Variables|Default|SetInvincible true)
  (Utilities|FlowControl|Delay Knockout%20Duration)
  (Variables|Default|SetKnockedout false)
  (Variables|Default|SetInvincible false))

(event EventBeginPlay
  (Utilities|FlowControl|Delay 0.1 :!label _label)
  (CallFunction|AnyDamageEvent 1e+01 true false 1.0)
  (goto _label))

(event Collision|EventActorBeginOverlap
  (params (OtherActor :type Actor%20Object%20Reference)))

(event EventTick
  (params (DeltaSeconds :type Float%20%28single-precision%29)))

(fn ConstructionScript)

(fn TakeDamage
  (params (Damage :type Float%20%28single-precision%29) (Ignore%20Shield :type Boolean) (Ignore%20Invincible :type Boolean))
  (bind _invincible (Variables|Default|GetInvincible))
  ;[0.2127 1 0.7675] Check for invincibility
  (Rendering|Debug|DrawDebugString (Transformation|GetWorldLocation (Variables|Default|GetInvincibleOverview)) (Utilities|String|ToString(Boolean) _invincible) 0 "(R=1.000000,G=0.000000,B=0.001355,A=1.000000)" 0.5)
  (if (not (and _invincible (not Ignore%20Invincible)))
    ;[0.4531 0.3237 0.2498] Reduce damage from shield
    (bind _shield (Utilities|GetShield)
      (:Out
        ;[0.6531 1 0.7187] SetHealth
        (if Ignore%20Shield
          (bind _health (Utilities|GetHealth)
            (:Out
              (Utilities|SetHealth (- _health Damage)
                (:Out
                  _))))
          (else
            (bind _health_2 (Utilities|GetHealth)
              (:Out
                (Utilities|SetHealth (- _health_2 (Math|Float|Clamp(Float) (- Damage _shield) 0.0 Damage))
                  (:Out
                    _))))))
        (Rendering|Debug|DrawDebugString (Transformation|GetWorldLocation (Variables|Default|GetHealthOverview)) (Utilities|String|ToString(Float) (stale _health)) 0 "(R=0.000000,G=1.000000,B=0.004274,A=1.000000)" 0.5)
        ;[0.4077 0.6619 1] SetShield
        (if (not Ignore%20Shield)
          (bind _shield_2 (Utilities|GetShield)
            (:Out
              (Utilities|SetShield (- _shield_2 Damage)
                (:Out
                  (Rendering|Debug|DrawDebugString (Transformation|GetWorldLocation (Variables|Default|GetShieldOverview)) (Utilities|String|ToString(Float) (stale _shield)) 0 "(R=0.000000,G=0.670315,B=1.000000,A=1.000000)" 0.5))))))))))