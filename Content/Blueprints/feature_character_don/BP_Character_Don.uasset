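; Character Blueprint for Don that manages health, temporary forcefield invulnerability and timed knockouts.
; Damage events lower clamped health unless the forcefield is up and can start a new forcefield; knockback damage also triggers a knockout when the hit lands.
; Tick clears both states by comparing stored expiry times to game time, then draws health and active states as debug text.
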(event Custom|Take_Any_Damage_Event
  (params (Damage :type Float%20%28single-precision%29) (Forcefield%20Duration :type Float%20%28single-precision%29))
  ;[1 1 1] Event when to take damage without status effect
  (Utilities|TakeDamage Damage Forcefield%20Duration))

(event Custom|Take_Knockback_Damage_Event
  (params (Damage :type Float%20%28single-precision%29) (Forcefield%20Duration :type Float%20%28single-precision%29) (Knockback%20Duration :type Float%20%28single-precision%29))
  ;[1 1 1] Event when to take damage with knockback status effect
  (Utilities|TakeDamage Damage Forcefield%20Duration
    (:Return
      (Utilities|TakeKnockback Knockback%20Duration))))

(event EventTick
  (params (DeltaSeconds :type Float%20%28single-precision%29))
  (bind _returnvalue (Utilities|Time|GetTimeSeconds))
  ;[1 1 1] Solves when to turn off godemode(forcefield) or when to restore from the knockout
  (if (<= (Variables|Default|GetGod_Time) _returnvalue)
    (Variables|Default|SetGod false))
  (if (<= (Variables|Default|GetKnockout_Time) _returnvalue)
    (Variables|Default|SetKnockout false))
  ;[1 1 1] debug drawings
  (Utilities|FlowControl|Sequence
    (:then_0
      (Rendering|Debug|DrawDebugString (Transformation|GetWorldLocation (Variables|Default|GetDebug%20draw%20Health)) (Utilities|String|ToString(Float) (Variables|Default|GetHealth)) 0 "(R=0.000000,G=1.000000,B=0.131249,A=1.000000)"))
    (:then_1
      (if (Variables|Default|GetGod)
        (Rendering|Debug|DrawDebugString (Transformation|GetWorldLocation (Variables|Default|GetDebug%20draw%20Forcefield)) "Godded" 0 "(R=0.000000,G=0.448144,B=1.000000,A=1.000000)")))
    (:then_2
      (if (Variables|Default|GetKnockout)
        (Rendering|Debug|DrawDebugString (Transformation|GetWorldLocation (Variables|Default|GetDebug%20draw%20Knockout)) "Knocked out" 0 "(R=1.000000,G=0.000000,B=0.000000,A=1.000000)")))))

(fn ConstructionScript)

(fn SetHealth
  (params (New%20Value :type Float%20%28single-precision%29))
  (bind _output_get (Variables|Default|SetHealth (Math|Float|Clamp(Float) New%20Value 0.0 1e+02)))
  (return _output_get))

(fn GetHealth
  (return (Variables|Default|GetHealth)))