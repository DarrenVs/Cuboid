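; BP_Hexcoin_Spawn is a spawner actor that places a Hexcoin at a random point inside its Spawn Area box.
; BeginPlay calls SpawnCoin, which adds a Child Actor Component at a random relative transform built from the box's relative location and extent.
; The component is stored in Coin so RemoveCoin can destroy it, though nothing in this Blueprint calls RemoveCoin.
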(event EventBeginPlay
  ;[1 1 1] Calls 'Spawn Coin'-function on begin play
  (CallFunction|SpawnCoin))

(event Collision|EventActorBeginOverlap
  (params (OtherActor :type Actor%20Object%20Reference)))

(event EventTick
  (params (DeltaSeconds :type Float%20%28single-precision%29)))

(fn ConstructionScript)

(fn SpawnCoin
  (bind _spawn_area (Variables|Default|GetSpawn%20Area))
  ;[1 1 1] Spawns Hexcoins at a random point within the Spawn Area
  (bind _returnvalue (AddComponent|AddChildActorComponent false (Math|Conversions|ToTransform(Vector) (Math|Random|RandomPointinBoundingBox (Variables|/Script/Engine.SceneComponent|GetRelativeLocation _spawn_area) (Variables|/Script/Engine.BoxComponent|GetBoxExtent _spawn_area)))))
  (Variables|Default|SetCoin _returnvalue))

(fn RemoveCoin
  (Components|DestroyComponent (Variables|Default|GetCoin)))