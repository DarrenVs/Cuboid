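; BP_AudioBarVisualizer is an audio visualizer actor that displays a row of cube bars whose heights follow audio values.
; The construction script adds evenly spaced instances to the Cubes instanced mesh along local X and stores their indices in Bars.
; Every Tick, it reads the matching AudioManager.AudioVariables entry for each bar and applies it as clamped Z scale, keeping location and rotation.
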(event EventBeginPlay)

(event Collision|EventActorBeginOverlap
  (params (OtherActor :type Actor%20Object%20Reference)))

(event EventTick
  (params (DeltaSeconds :type Float%20%28single-precision%29))
  (CallFunction|UpdateBars))

(fn ConstructionScript
  (CallFunction|CreateBars))

(fn CreateBars
  (for _index (range 0 (Variables|Default|GetBarAmount))
    (bind _returnvalue (Components|InstancedStaticMesh|AddInstance (Variables|Default|GetCubes) (Math|Transform|MakeTransform (Math|Vector|MakeVector (Math|Conversions|ToFloat(Integer) (* _index 100)) 0.0 0.0))))
    (Utilities|Array|Add (Variables|Default|GetBars) _returnvalue)))

(fn UpdateBars
  (for (_array_element _array_index) (Variables|Default|GetBars)
    (Components|InstancedStaticMesh|UpdateInstanceTransform (Variables|Default|GetCubes) _array_element (Math|Transform|MakeTransform (.Location (Math|Transform|BreakTransform (.OutInstanceTransform (Components|InstancedStaticMesh|GetInstanceTransform (Variables|Default|GetCubes) _array_element false)))) (.Rotation (Math|Transform|BreakTransform (.OutInstanceTransform (Components|InstancedStaticMesh|GetInstanceTransform (Variables|Default|GetCubes) _array_element false)))) (Math|Vector|MakeVector 1.0 1.0 (Math|Float|Clamp(Float) (Utilities|Array|Get(acopy) (Variables|/Game/Blueprints/BP_AudioManager.BP_AudioManager_C|GetAudioVariables (Variables|Default|GetAudioManager)) _array_index) 0.0 1e+02))) false true false)))