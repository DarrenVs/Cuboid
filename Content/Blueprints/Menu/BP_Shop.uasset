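; In-game shop actor with a widget that sells an armour upgrade through a hover-to-confirm (dwell) button.
; Each Tick, hovering the button with enough BP_Character Score fills a progress bar over StareTime; leaving resets it.
; A full bar passes through a Gate to set BP_Health_Pawn's Armour and disable the button.
; The cost is only checked against Score, never deducted here.
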(event EventTick
  (params (DeltaSeconds :type Float%20%28single-precision%29))
  (bind _aswbp_ingame_shop (Utilities|Casting|CastToWBP_IngameShop (UserInterface|GetUserWidgetObject (Variables|Default|GetShop))))
  (if (Widget|IsHovered (Variables|/Game/Widget/WBP_IngameShop.WBP_IngameShop_C|GetButton_80 _aswbp_ingame_shop))
    (bind _outactors (Actor|GetAllActorsOfClass "/Game/Blueprints/feature_score_system/BP_Character.BP_Character_C"))
    (if (>= (Variables|/Game/Blueprints/feature_score_system/BP_Character.BP_Character_C|Getscore (Utilities|Array|Get(acopy) _outactors)) (Variables|Default|GetArmourCost))
      (bind _output_get (Variables|Default|SetLoadBarProg (+ (Variables|Default|GetLoadBarProg) (/ DeltaSeconds (Variables|Default|GetStareTime)))))
      (Progress|SetPercent (Variables|/Game/Widget/WBP_IngameShop.WBP_IngameShop_C|GetProgressBar_119 _aswbp_ingame_shop) _output_get)
      (Utilities|FlowControl|Sequence
        (:then_0
          (goto _label Open))
        (:then_1
          (if (>= (Variables|/Script/UMG.ProgressBar|GetPercent (Variables|/Game/Widget/WBP_IngameShop.WBP_IngameShop_C|GetProgressBar_119 _aswbp_ingame_shop)) 1.0)
            (Utilities|FlowControl|Gate true :!label _label
              (:Exit
                (bind _outactors_2 (Actor|GetAllActorsOfClass "/Game/Blueprints/feature_pawn_health/BP_Health_Pawn.BP_Health_Pawn_C"))
                (bind _asbp_health_pawn (Utilities|Casting|CastToBP_Health_Pawn (Utilities|Array|Get(acopy) _outactors_2)))
                (Variables|/Game/Blueprints/feature_pawn_health/BP_Health_Pawn.BP_Health_Pawn_C|SetArmour _asbp_health_pawn 5.0)
                (bind _aswbp_ingame_shop_2 (Utilities|Casting|CastToWBP_IngameShop (UserInterface|GetUserWidgetObject (Variables|Default|GetShop))))
                (Widget|SetIsEnabled (Variables|/Game/Widget/WBP_IngameShop.WBP_IngameShop_C|GetButton_80 _aswbp_ingame_shop_2) false)))))))
    (else
      (bind _output_get_2 (Variables|Default|SetLoadBarProg 0.0))
      (Progress|SetPercent (Variables|/Game/Widget/WBP_IngameShop.WBP_IngameShop_C|GetProgressBar_119 _aswbp_ingame_shop) _output_get_2)
      (goto _label Close))))

(fn ConstructionScript)