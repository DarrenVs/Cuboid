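; Main menu actor that starts the game through gaze-and-hold selection on a WBP_MainMenu widget.
; Tick fills the widget's progress bar over WaitTime while it is hovered and resets it otherwise.
; A Gate, open only during hover, passes once the bar is full to play the door animation and sound.
; Delays then stagger setting StartMoving on BP_MenuCharacterMov and opening the ChunkGeneration level.
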(event EventTick
  (params (DeltaSeconds :type Float%20%28single-precision%29))
  (bind _aswbp_main_menu (Utilities|Casting|CastToWBP_MainMenu (UserInterface|GetUserWidgetObject (Variables|Default|GetWidget)))) ; Get the widget blueprint
  (if (Widget|IsHovered _aswbp_main_menu)
    (bind _output_get (Variables|Default|SetloadingBarProgress (+ (Variables|Default|GetloadingBarProgress) (/ DeltaSeconds (Variables|Default|GetWaitTime)))))
    ;[1 1 1] Set the loading bar widget property
    (Progress|SetPercent (Variables|/Game/Widget/WBP_MainMenu.WBP_MainMenu_C|GetProgressBar_57 _aswbp_main_menu) _output_get)
    (Utilities|FlowControl|Sequence
      (:then_0
        (goto _label Open))
      (:then_1
        (if (>= (Variables|/Script/UMG.ProgressBar|GetPercent (Variables|/Game/Widget/WBP_MainMenu.WBP_MainMenu_C|GetProgressBar_57 _aswbp_main_menu)) 1.0)
          (Utilities|FlowControl|Gate true :!label _label ; When the loading bar is full. Go through the exit
            (:Exit
              ;[1 1 1] Start the door animation and play the sound
              (Audio|Components|Audio|Play (Variables|/Script/Engine.SkeletalMeshActor|GetSkeletalMeshComponent (Variables|Default|GetDoor)) false) ; Start the door animation
              (Components|Activation|Activate (Variables|/Script/Engine.AmbientSound|GetAudioComponent (Variables|Default|GetDoorSound)) false)
              (Utilities|FlowControl|Delay 3.0)
              (bind _asbp_menu_character_mov (Utilities|Casting|CastToBP_MenuCharacterMov (Variables|Default|GetCharacterMove)))
              (Variables|/Game/Blueprints/MainMenu_CharacterMovement/BP_MenuCharacterMov.BP_MenuCharacterMov_C|SetStartMoving _asbp_menu_character_mov true)
              (Utilities|FlowControl|Delay 4.5)
              (Game|OpenLevel(byName) "ChunkGeneration") ; Start the game level
            )))))
    (else
      (bind _output_get_2 (Variables|Default|SetloadingBarProgress 0.0))
      (Progress|SetPercent (Variables|/Game/Widget/WBP_MainMenu.WBP_MainMenu_C|GetProgressBar_57 _aswbp_main_menu) _output_get_2)
      (goto _label Close))))

(fn ConstructionScript)