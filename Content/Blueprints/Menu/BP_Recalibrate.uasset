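; BP_Recalibrate is a gaze-activated menu actor that recalibrates the VR headset's orientation and position.
; While its WBP_Recalibrate widget is hovered, Tick fills a progress bar over ClickTime; losing hover empties it and closes a Gate.
; A full bar passes through the Gate to a two-second Delay, then ResetOrientationAndPosition.
; The Gate reopens every hovered tick, so continued hovering repeats the reset after each delay.
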(event EventTick
  (params (DeltaSeconds :type Float%20%28single-precision%29))
  (bind _aswbp_recalibrate (Utilities|Casting|CastToWBP_Recalibrate (UserInterface|GetUserWidgetObject (Variables|Default|GetWidget)))) ; Get the widget blueprint
  (if (Widget|IsHovered _aswbp_recalibrate)
    ;[1 1 1] Set loading bar value
    (bind _output_get (Variables|Default|SetLoadingBarProgress (+ (Variables|Default|GetLoadingBarProgress) (/ DeltaSeconds (Variables|Default|GetClickTime)))))
    (Progress|SetPercent (Variables|/Game/Widget/WBP_Recalibrate.WBP_Recalibrate_C|GetProgressBar_57 _aswbp_recalibrate) _output_get)
    (Utilities|FlowControl|Sequence
      (:then_0
        (goto _label Open))
      (:then_1
        (if (>= (Variables|/Script/UMG.ProgressBar|GetPercent (Variables|/Game/Widget/WBP_Recalibrate.WBP_Recalibrate_C|GetProgressBar_57 _aswbp_recalibrate)) 1.0)
          (Utilities|FlowControl|Gate true :!label _label ; Wait till the loading bar is full
            (:Exit
              ;[1 1 1] Wait for the recalibration of the headset
              (Utilities|FlowControl|Delay 2.0)
              (Class|HeadMountedDisplayFunctionLibrary|ResetOrientationandPosition 0.0 "OrientationAndPosition"))))))
    (else
      (bind _output_get_2 (Variables|Default|SetLoadingBarProgress 0.0))
      (Progress|SetPercent (Variables|/Game/Widget/WBP_Recalibrate.WBP_Recalibrate_C|GetProgressBar_57 _aswbp_recalibrate) _output_get_2)
      (goto _label Close))))

(fn ConstructionScript)